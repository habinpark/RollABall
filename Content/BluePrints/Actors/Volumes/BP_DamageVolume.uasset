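; BP_DamageVolume is a trigger volume that ends the game on its first overlap rather than applying damage.
; The overlap runs once, without checking the overlapping actor, and sets IsEnd on player 0's BP_PlayerPawn.
; It then fades the camera to black, waits briefly, adds UI_EndScreen and shows the mouse cursor.
; A current-level reload remains in the graph but is unconnected.
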(event OnComponentBeginOverlap(Trigger)
  (params (OverlappedComponent :type Primitive%20Component%20Object%20Reference) (OtherActor :type Actor%20Object%20Reference) (OtherComp :type Primitive%20Component%20Object%20Reference) (OtherBodyIndex :type Integer) (bFromSweep :type Boolean) (SweepResult :type Hit%20Result%20Structure%20%28by%20ref%29))
  (bind _returnvalue (Math|Float|MakeLiteralFloat 1.0))
  (Utilities|FlowControl|DoOnce false
    (:Completed
      (bind _asbp_player_pawn (Utilities|Casting|CastToBP_PlayerPawn (Game|Player|GetPlayerPawn 0)))
      (Variables|/Game/BluePrints/BP_PlayerPawn.BP_PlayerPawn_C|SetIsEnd _asbp_player_pawn true)
      (CameraFades|StartCameraFade (Game|GetPlayerCameraManager 0) 0.0 1.0 _returnvalue "(R=0.000000,G=0.000000,B=0.000000,A=1.000000)" false false)
      (Utilities|FlowControl|Delay _returnvalue)
      ;[1 1 1] addsEndscreenWidget
      (bind _returnvalue_2 (UserInterface|CreateWidget "/Game/BluePrints/UI_EndScreen.UI_EndScreen_C"))
      (UserInterface|Viewport|AddtoViewport _returnvalue_2 0)
      (Variables|/Script/Engine.PlayerController|SetbShowMouseCursor (Game|GetPlayerController 0) true))))

(event EventBeginPlay)

(event Collision|EventActorBeginOverlap
  (params (OtherActor :type Actor%20Object%20Reference)))

(event EventTick
  (params (DeltaSeconds :type Float%20%28single-precision%29)))

(fn ConstructionScript)