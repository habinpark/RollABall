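; BP_WinVolume is a volume that completes the level when the player overlaps it and no BP_Crystal actors remain.
; Completion opens the next entry in the LevelName array, or quits the game on the final level.
; Progression depends on GetCurrentLevelIndex, meant to find the current level's name in that array.
; Its return step is never executed as wired, so that lookup does not reach the caller.
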(event Collision|EventActorBeginOverlap
  (params (OtherActor :type Actor%20Object%20Reference))
  (Utilities|IsPlayer OtherActor
    (:IsPlayer
      (if (not (CallFunction|AnyCrystalsRemaining))
        (CallFunction|CompleteLevel)))))

(fn ConstructionScript)

(fn AnyCrystalsRemaining
  (bind _outactors (Actor|GetAllActorsOfClass "/Game/BluePrints/Actors/Collectables/BP_Crystal.BP_Crystal_C"))
  (return (> (Utilities|Array|Length _outactors) 0)))

(fn CompleteLevel
  (if (CallFunction|IsFinalLevel)
    (Game|QuitGame 0 "Quit")
    (else
      (CallFunction|LoadNextLevel))))

(fn GetCurrentLevelIndex
  (bind _returnvalue (Game|GetCurrentLevelName true)))

(fn IsFinalLevel
  (return (== (Utilities|Array|LastIndex (Variables|Default|GetLevelName)) (CallFunction|GetCurrentLevelIndex))))

(fn LoadNextLevel
  (Game|OpenLevel(byName) (CallFunction|GetNextLevelName)))

(fn GetNextLevelName
  (return (Utilities|Array|Get(acopy) (Variables|Default|GetLevelName) (+ 1 (CallFunction|GetCurrentLevelIndex)))))