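; BP_CannonSlow is a cannon actor that automatically and repeatedly fires slow projectiles from BeginPlay onward.
; After each FireRate delay, it spawns a BP_ProjectileSlow at ProjectileSpawnPoint, scaled by ProjectileScale.
; A timeline then animates the CannonBarrel's relative location, and its Cannon Fired event loops back to the delay for the next shot.
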(event EventBeginPlay
  (Utilities|FlowControl|Delay (Variables|CannonProperties|GetFire%20Rate) :!label _label)
  (CallFunction|SpawnProjectile)
  (bind _cannon_fire_ (Timeline|Timeline_0 PlayFromStart)
    (:Update
      (CallFunction|MoveCannonBarrel _cannon_fire_))
    (:Cannon%20Fired
      (goto _label))))

(fn ConstructionScript)

(fn SpawnProjectile
  (bind _projectilespawnpoint (Variables|Default|GetProjectileSpawnPoint))
  (Game|SpawnActorfromClass "/Game/BluePrints/Actors/Projectiles/BP_ProjectileSlow.BP_ProjectileSlow_C" (Math|Transform|MakeTransform (Transformation|GetWorldLocation _projectilespawnpoint) (Transformation|GetWorldRotation _projectilespawnpoint) (Math|Conversions|ToVector(Float) (Variables|CannonProperties|GetProjectile%20Scale))) "Undefined" 0 0))

(fn MoveCannonBarrel
  (params (NewLocation_Y :type Float%20%28single-precision%29))
  (Transformation|SetRelativeLocation (Variables|Default|GetCannon_Barrel) (Math|Vector|MakeVector 0.0 NewLocation_Y 0.0) false false))