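; BP_Crystal is a collectable crystal actor that flies into the player and vanishes when the player overlaps it.
; On overlap it caches its starting location, scale and point light intensity, then plays a timeline with a separate track for each.
; The tracks lerp it toward the player's live position, shrink it and fade the light to zero.
; The actor destroys itself when the timeline finishes.
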(event Collision|EventActorBeginOverlap
  (params (OtherActor :type Actor%20Object%20Reference))
  (Utilities|IsPlayer OtherActor
    (:IsPlayer
      (CallFunction|StoreStartingValues)
      (bind (_direction _collection_progress _scale_progress _lightintensity) (Timeline|Alpha%20Blend%20Timeline Play)
        (:Update
          (CallFunction|MovetoPlayer _collection_progress)
          (CallFunction|ShrinkScale _scale_progress)
          (CallFunction|DecreaseLightIntensity _lightintensity))
        (:Finished
          (Actor|DestroyActor))))))

(fn ConstructionScript)

(fn MovetoPlayer
  (params (Alpha :type Float%20%28single-precision%29))
  (Transformation|SetActorLocation (Math|Vector|Lerp(Vector) (Variables|Default|Getstart%20location) (Transformation|GetActorLocation (Game|Player|GetPlayerPawn 0)) Alpha) false false))

(fn StoreStartingValues
  (Variables|Default|Setstart%20location (Transformation|GetActorLocation))
  (Variables|Default|SetStartScale (Transformation|GetActorScale3D))
  (Variables|Default|SetStartLightIntensity (Variables|/Script/Engine.LightComponentBase|GetIntensity (Variables|Default|GetPointLight))))

(fn ShrinkScale
  (params (Alpha :type Float%20%28single-precision%29))
  (Transformation|SetActorScale3D (Math|Vector|Lerp(Vector) (Variables|Default|GetStartScale) (Variables|Default|GetScaleEnd) Alpha)))

(fn DecreaseLightIntensity
  (params (Alpha :type Float%20%28single-precision%29))
  (Rendering|Components|Light|SetIntensity (Variables|Default|GetPointLight) (Math|Float|Lerp (Variables|Default|GetStartLightIntensity) 0.0 Alpha)))