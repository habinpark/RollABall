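; Player pawn that rolls a physics sphere by torque, explodes on any damage and restarts the level.
; Forward/back input applies equal X and Y torque, right/left input is empty, and mouse axes steer controller yaw and pitch.
; BeginPlay fades in from black; the RestartLevel macro uses DoOnce to fade out, wait, then reload the current level by name.
; End-screen widget and DestroyActor logic are left unconnected.
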(event EventBeginPlay
  (bind _returnvalue (Math|Float|MakeLiteralFloat 1.0))
  (CameraFades|StartCameraFade (Game|GetPlayerCameraManager 0) 1.0 0.0 _returnvalue "(R=0.000000,G=0.000000,B=0.000000,A=1.000000)" false false)
  (Utilities|FlowControl|Delay _returnvalue))

(event Game|Damage|EventAnyDamage
  (params (Damage :type Float%20%28single-precision%29) (DamageType :type Damage%20Type%20Object%20Reference) (InstigatedBy :type Controller%20Object%20Reference) (DamageCauser :type Actor%20Object%20Reference))
  (Game|SpawnActorfromClass "/Game/StarterContent/Blueprints/Blueprint_Effect_Explosion.Blueprint_Effect_Explosion_C" (Transformation|GetActorTransform) "Undefined" 0 0)
  (Utilities|RestartLevel))

(event Input|AxisEvents|InputAxisMoveFowards/Backwards
  (params (AxisValue :type Float%20%28single-precision%29))
  (Variables|Default|SetTorqueSpeed 5e+01)
  (Class|PrimitiveComponent|AddTorqueinRadians (Variables|Default|GetSphere) (Math|Vector|MakeVector (* (stale Input|AxisEvents|InputAxisMoveRight/Left AxisValue) (Variables|Default|GetTorqueSpeed)) (* AxisValue (Variables|Default|GetTorqueSpeed)) 0.0) "None" true))

(event Input|AxisEvents|InputAxisMoveRight/Left
  (params (AxisValue :type Float%20%28single-precision%29)))

(event Input|AxisEvents|InputAxisLookUp
  (params (AxisValue :type Float%20%28single-precision%29))
  ;[1 1 1] MouseInput
  (Pawn|Input|AddControllerPitchInput AxisValue))

(event Input|AxisEvents|InputAxisTurn
  (params (AxisValue :type Float%20%28single-precision%29))
  ;[1 1 1] MouseInput
  (Pawn|Input|AddControllerYawInput AxisValue))

(fn ConstructionScript)